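; SpawnerCubeBP is a spawner that builds a grid of Cube_BP actors from its own location on BeginPlay.
; An outer loop spawns cubes along the left direction, and a nested loop extends a line forward from each one, both bounded by Row.
; Each new cube's LeftLocation or FrontLocation supplies the next spawn position, so placement chains from the cubes themselves.
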(event `self.ReceiveBeginPlay`
  (set `self.Next` (`self.K2_GetActorLocation`))
  (for _ (range (+ (`self.Row`) 1))
    (bind _returnvalue (`|SpawnActorFromClass` "/Game/Blueprints/Cube_BP.Cube_BP_C" (`KismetMathLibrary.Conv_VectorToTransform` (`self.Next`)) "Undefined" "OverrideRootScale" null null))
    (set `self.Next` (`/Game/Blueprints/Cube_BP.LeftLocation` _returnvalue))
    (set `self.NextFron` (`/Game/Blueprints/Cube_BP.FrontLocation` _returnvalue))
    (for _ (range (+ (`self.Row`) 1))
      (bind _returnvalue_2 (`|SpawnActorFromClass` "/Game/Blueprints/Cube_BP.Cube_BP_C" (`KismetMathLibrary.Conv_VectorToTransform` (`self.NextFron`)) "Undefined" "OverrideRootScale" null null))
      (set `self.NextFron` (`/Game/Blueprints/Cube_BP.FrontLocation` _returnvalue_2)))))

(fn `UserConstructionScript`)